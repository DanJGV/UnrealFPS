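; BP_MovableObject is an actor that moves continuously around a looping path of node actors.
; Each Tick it lerps its location toward the current node using delta seconds as alpha, giving an eased approach without sweeping.
; Once within a small distance of that node, it advances to the next index and wraps back to the first after the last.
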(event `self.ReceiveBeginPlay`)

(event `self.ReceiveTick`
  (params (DeltaSeconds :type "Float (single-precision)"))
  (bind _returnvalue (`self.K2_GetActorLocation`))
  (bind _index (`self.index`))
  (bind _returnvalue_2 (`self.K2_GetActorLocation` (`|GetArrayItem` (`self.nodes`) (`self.index`))))
  (`self.K2_SetActorLocation` (`KismetMathLibrary.VLerp` _returnvalue _returnvalue_2 DeltaSeconds))
  (if (<= (`KismetMathLibrary.Vector_Distance` _returnvalue _returnvalue_2) 100.0)
    (`/Engine/EditorBlueprintResources/StandardMacros.IncrementInt` _index
      (:`  `
        (if (>= _index (`KismetArrayLibrary.Array_Length` (`self.nodes`)))
          (set `self.index` 0))))))

(fn `UserConstructionScript`)