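; Bullet actor that scores points for the player by destroying actors it overlaps that carry a configurable tag.
; Tick accumulates elapsed time and destroys the bullet once its lifetime runs out.
; Each tagged overlap destroys that actor, but not the bullet, and increments Score on the player's BP_MyCharacter.
; When Score equals the character's GoalScore, it opens the GameOverScreen level.
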(event `self.ReceiveTick`
  (params (DeltaSeconds :type "Float (single-precision)"))
  ;[1 1 1] Bullet travel
  (set `self.elapsed` (+ DeltaSeconds (`self.elapsed`)))
  (if (>= (`self.elapsed`) (`self.lifetime`))
    (`self.K2_DestroyActor`)))

(event `self.ReceiveActorBeginOverlap`
  (params (OtherActor :type "Actor Object Reference"))
  (if (`self.ActorHasTag` OtherActor (`self.tag`))
    (`self.K2_DestroyActor` OtherActor)
    (bind _asbp_my_character (cast `/Game/Blueprints/BP_MyCharacter` (`GameplayStatics.GetPlayerCharacter` 0)))
    (bind _score (`/Game/Blueprints/BP_MyCharacter.score` _asbp_my_character))
    (`/Engine/EditorBlueprintResources/StandardMacros.IncrementInt` _score
      (:`  `
        (if (== _score (`/Game/Blueprints/BP_MyCharacter.goalScore` _asbp_my_character))
          (`GameplayStatics.OpenLevel` "GameOverScreen"))))))

(event `self.ReceiveHit`
  (params (MyComp :type "PrimitiveComponent Object Reference") (Other :type "Actor Object Reference") (OtherComp :type "PrimitiveComponent Object Reference") (bSelfMoved :type Boolean) (HitLocation :type "Vector Structure") (HitNormal :type "Vector Structure") (NormalImpulse :type "Vector Structure") (Hit :type "HitResult Structure (by ref)")))

(fn `UserConstructionScript`)