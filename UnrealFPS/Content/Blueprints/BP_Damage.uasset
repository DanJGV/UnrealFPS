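; BP_Damage is a hazard volume that hurts the player character when it enters the Box trigger.
; On begin overlap it calls PlayerDoT on BP_MyCharacter and subtracts a fixed amount from CurrentHealth, loading the GameOverScreen level at zero or below.
; On end overlap it calls PlayerNotCoT on the character.
; The damage branch is hardwired true, and a leftover debug print is never run.
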(event `self.ReceiveActorBeginOverlap`
  (params (OtherActor :type "Actor Object Reference")))

(event `self.ReceiveTick`
  (params (DeltaSeconds :type "Float (single-precision)")))

(event `self.ReceiveBeginPlay`)

(event `self.Box.OnComponentBeginOverlap`
  (params (OverlappedComponent :type "PrimitiveComponent Object Reference") (OtherActor :type "Actor Object Reference") (OtherComp :type "PrimitiveComponent Object Reference") (OtherBodyIndex :type Integer) (bFromSweep :type Boolean) (SweepResult :type "HitResult Structure (by ref)"))
  (bind _asbp_my_character (cast `/Game/Blueprints/BP_MyCharacter` OtherActor))
  (`/Game/Blueprints/BP_MyCharacter.PlayerDoT` _asbp_my_character)
  (if true
    (bind _currenthealth (`/Game/Blueprints/BP_MyCharacter.currentHealth` _asbp_my_character))
    (set `/Game/Blueprints/BP_MyCharacter.currentHealth` (- _currenthealth 5.0) _asbp_my_character)
    (if (<= _currenthealth 0.0)
      (`GameplayStatics.OpenLevel` "GameOverScreen"))))

(event `self.Box.OnComponentEndOverlap`
  (params (OverlappedComponent :type "PrimitiveComponent Object Reference") (OtherActor :type "Actor Object Reference") (OtherComp :type "PrimitiveComponent Object Reference") (OtherBodyIndex :type Integer))
  (bind _asbp_my_character (cast `/Game/Blueprints/BP_MyCharacter` OtherActor))
  (`/Game/Blueprints/BP_MyCharacter.playerNotCoT` _asbp_my_character))

(fn `UserConstructionScript`)